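; BP_ENARIS is the hookshot actor for a 2D action game, attaching to surfaces and pulling the player toward them.
; A Box hit on either of two custom object channels flags the Player as connected, stores the Box location as end point and calls REFHookshotCancelInConnected.
; While connected, Tick launches the Player along the normalized X/Z direction to that point, scaled by HookshotVelocityRatio.
; DrawHookshotString runs each Tick but is empty, its debug line trace disconnected.
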(event OnComponentHit(Box)
  (params (HitComponent :type Primitive%20Component%20Object%20Reference) (OtherActor :type Actor%20Object%20Reference) (OtherComp :type Primitive%20Component%20Object%20Reference) (NormalImpulse :type Vector :default "0, 0, 0") (Hit :type Hit%20Result%20Structure%20%28by%20ref%29))
  (bind _returnvalue (Collision|GetCollisionObjectType OtherComp))
  (bind _player (Variables|Default|GetPlayer))
  (if (or (Utilities|Enum|Equal(Enum) _returnvalue "ECC_GameTraceChannel3") (Utilities|Enum|Equal(Enum) _returnvalue "ECC_GameTraceChannel5"))
    (Variables|/Game/2DAction/Blueprints/BP_Player_2D_PaperZD.BP_Player_2D_PaperZD_C|SetIs%20Hookshot%20Connected _player true)
    (Variables|/Game/2DAction/Blueprints/BP_Player_2D_PaperZD.BP_Player_2D_PaperZD_C|SetHookshot%20End%20Point _player (Transformation|GetWorldLocation (Variables|Default|GetBox)))
    (Default|REFHookshotCancelinConnected (Variables|Default|GetPlayer))))

(event EventBeginPlay)

(event Collision|EventActorBeginOverlap
  (params (OtherActor :type Actor%20Object%20Reference)))

(event EventTick
  (params (DeltaSeconds :type Float%20%28single-precision%29))
  (CallFunction|MovebyHookshot)
  (CallFunction|DrawHookshotString))

(fn ConstructionScript)

(fn DrawHookshotString)

(fn MovebyHookshot
  (bind _player (Variables|Default|GetPlayer))
  (bind _player_2 (Variables|Default|GetPlayer))
  (bind _player_3 (Variables|Default|GetPlayer))
  (bind _hookshot_velocity_ratio (Variables|/Game/2DAction/Blueprints/BP_Player_2D_PaperZD.BP_Player_2D_PaperZD_C|GetHookshot%20Velocity%20Ratio _player))
  (bind _capsulecomponent (Variables|/Script/Engine.Character|GetCapsuleComponent _player_2))
  (bind _hookshot_end_point (Variables|/Game/2DAction/Blueprints/BP_Player_2D_PaperZD.BP_Player_2D_PaperZD_C|GetHookshot%20End%20Point _player_3))
  (bind _returnvalue (Transformation|GetWorldLocation _capsulecomponent))
  (bind _returnvalue_2 (- _hookshot_end_point _returnvalue))
  (bind _returnvalue_3 (Math|Vector|Normalize _returnvalue_2))
  (if (Variables|/Game/2DAction/Blueprints/BP_Player_2D_PaperZD.BP_Player_2D_PaperZD_C|GetIs%20Hookshot%20Connected (Variables|Default|GetPlayer))
    (Character|LaunchCharacter (Variables|Default|GetPlayer) (Math|Vector|MakeVector (* (.x _returnvalue_3) _hookshot_velocity_ratio) 0.0 (* _hookshot_velocity_ratio (.z _returnvalue_3))) false false)))