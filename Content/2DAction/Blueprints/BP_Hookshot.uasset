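; BP_Hookshot is the hookshot actor in a 2D action game, detecting when its Box component hits an attachable collision type.
; On a hit with either of two custom object channels, it marks the Player as connected, passes the Box location as the endpoint and calls REFHookshotCancelInConnected.
; DrawHookshotString fakes the rope with a short-lived debug line trace from the Box to the Player's capsule; nothing in this Blueprint calls it.
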(event OnComponentHit(Box)
  (params (HitComponent :type Primitive%20Component%20Object%20Reference) (OtherActor :type Actor%20Object%20Reference) (OtherComp :type Primitive%20Component%20Object%20Reference) (NormalImpulse :type Vector :default "0, 0, 0") (Hit :type Hit%20Result%20Structure%20%28by%20ref%29))
  (bind _returnvalue (Collision|GetCollisionObjectType OtherComp))
  (bind _player (Variables|Default|GetPlayer))
  (if (or (Utilities|Enum|Equal(Enum) _returnvalue "ECC_GameTraceChannel3") (Utilities|Enum|Equal(Enum) _returnvalue "ECC_GameTraceChannel5"))
    (Variables|/Game/2DAction/Blueprints/BP_Player_2D_PaperZD.BP_Player_2D_PaperZD_C|SetIs%20Hookshot%20Connected _player true)
    (Variables|/Game/2DAction/Blueprints/BP_Player_2D_PaperZD.BP_Player_2D_PaperZD_C|SetHookshot%20End%20Point _player (Transformation|GetWorldLocation (Variables|Default|GetBox)))
    (Default|REFHookshotCancelinConnected (Variables|Default|GetPlayer))))

(event EventBeginPlay)

(event Collision|EventActorBeginOverlap
  (params (OtherActor :type Actor%20Object%20Reference)))

(event EventTick
  (params (DeltaSeconds :type Float%20%28single-precision%29)))

(fn ConstructionScript)

(fn DrawHookshotString
  (Collision|LineTraceByChannel (Transformation|GetWorldLocation (Variables|Default|GetBox)) (Transformation|GetWorldLocation (Variables|/Script/Engine.Character|GetCapsuleComponent (Variables|Default|GetPlayer))) "TraceTypeQuery1" false 0 "ForDuration" true "(R=1.000000,G=0.000000,B=0.000000,A=1.000000)" "(R=0.000000,G=1.000000,B=0.000000,A=1.000000)" 0.01))